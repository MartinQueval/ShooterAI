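; AI controller for the ShooterAI module that runs the BT_SAIAI behavior tree on BeginPlay and reacts to AI perception.
; A perception update sets the hasSeenPlayer key to true on the blackboard looked up from the perceived actor, not the controller's own.
; A forgotten target only has its blackboard reference printed as text, and the key is never cleared here.
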(event OnTargetPerceptionUpdated(AIPerception)
  (params (Actor :type Actor%20Object%20Reference) (Stimulus :type AI%20Stimulus%20Structure))
  (AI|Components|Blackboard|SetValueasBool (AI|GetBlackboard Actor) (Utilities|Name|MakeLiteralName "hasSeenPlayer") true))

(event OnTargetPerceptionForgotten(AIPerception)
  (params (Actor :type Actor%20Object%20Reference))
  (for _array_element (Utilities|Array|MakeArray (AI|GetBlackboard Actor))
    (Development|PrintText (Utilities|Text|ToText(Object) _array_element))))

(event EventBeginPlay
  (AI|RunBehaviorTree "/Game/ShooterAI/AI/BT_SAIAI.BT_SAIAI"))

(event EventTick
  (params (DeltaSeconds :type Float%20%28single-precision%29)))

(fn ConstructionScript)