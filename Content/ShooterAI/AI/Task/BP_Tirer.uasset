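; BP_Tirer is a behavior tree task that makes an AI character fire one rifle shot at its target actor.
; It line-traces from the weapon muzzle toward the target with random spray, playing a shot sound and spawning a bullet-hole decal and Niagara trail.
; It applies fixed damage to any hit actor other than the shooter, waits for the firing-speed delay, then finishes as failed.
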(event EventReceiveExecuteAI
  (params (OwnerController :type AI%20Controller%20Object%20Reference) (ControlledPawn :type Pawn%20Object%20Reference))
  (bind _weapon_spray_range (Variables|Default|GetWeapon%20Spray%20Range))
  (bind _returnvalue (* _weapon_spray_range -1.0))
  ;[1 1 1] Weapon Trace
  (bind _asbp_saiaaicharacter (Utilities|Casting|CastToBP_SAIAAICharacter ControlledPawn))
  (bind _outhit (Collision|LineTraceByChannel (.location (Transformation|GetSocketTransform (Variables|/Game/ShooterAI/AI/BP_SAIAAICharacter.BP_SAIAAICharacter_C|GetWeapon _asbp_saiaaicharacter) "Muzzle" "RTS_World")) (+ (Transformation|GetActorLocation (Variables|/Script/ShooterAI.SAIAAICharacter|GetTargetActor _asbp_saiaaicharacter)) (Math|Vector|MakeVector (Math|Random|RandomFloatinRange _returnvalue _weapon_spray_range) (Math|Random|RandomFloatinRange _returnvalue _weapon_spray_range) (Math|Random|RandomFloatinRange _returnvalue _weapon_spray_range))) "TraceTypeQuery3" false 0 "None" true "(R=1.000000,G=0.006102,B=0.000000,A=0.800000)" "(R=0.000000,G=1.000000,B=0.000000,A=1.000000)" 0.5))
  (Audio|PlaySoundatLocation "/Game/ShooterAI/SOunds/MSSAI_RIfleShot.MSSAI_RIfleShot" (.location (Transformation|GetSocketTransform (Variables|/Game/ShooterAI/AI/BP_SAIAAICharacter.BP_SAIAAICharacter_C|GetWeapon _asbp_saiaaicharacter) "Muzzle" "RTS_World")) "0, 0, 0" 1.0 1.0 0.0 0 0 0 0)
  (Rendering|Decal|SpawnDecalatLocation "/Game/ShooterAI/Textures/Bullet_Hole_Material.Bullet_Hole_Material" (Math|Conversions|ToVector(Float) (Math|Random|RandomIntegerinRange 3 7)) (.Location (Collision|BreakHitResult _outhit)) (Math|Conversions|RotationFromXVector (.ImpactNormal (Collision|BreakHitResult _outhit))) 5.0)
  (bind _returnvalue_2 (Niagara|SpawnSystematLocation "/Game/ShooterAI/Effects/NSAI_BulletTrail_System.NSAI_BulletTrail_System" (.location (Transformation|GetSocketTransform (Variables|/Game/ShooterAI/AI/BP_SAIAAICharacter.BP_SAIAAICharacter_C|GetWeapon _asbp_saiaaicharacter) "Muzzle" "RTS_World"))))
  (Effects|Components|ParticleSystem|SetVectorParameter _returnvalue_2 "BeamEnd" (.TraceEnd (Collision|BreakHitResult _outhit)))
  (if true
    (if (!= _asbp_saiaaicharacter (.HitActor (Collision|BreakHitResult _outhit)))
      (Game|Damage|ApplyDamage (.HitActor (Collision|BreakHitResult _outhit)) 2e+01 0 0)
      (Utilities|FlowControl|Delay (Variables|Default|GetFiring%20Speed) :!label _label))
    (else
      (goto _label)))
  (AI|BehaviorTree|FinishExecute false))