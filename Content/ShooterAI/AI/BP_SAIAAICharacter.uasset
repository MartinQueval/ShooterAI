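; BP_SAIAAICharacter is an AI enemy character with a simple health system and a floating health bar.
; Any damage lowers Health, plays a 2D hitmarker sound and updates the UISAI_EnemyHealth progress bar in its widget component.
; At zero health the mesh switches to ragdoll physics and the actor is destroyed after a short delay.
; Every tick the health bar widget rotates to face the player camera.
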(event Game|Damage|EventAnyDamage
  (params (Damage :type Float%20%28single-precision%29) (DamageType :type Damage%20Type%20Object%20Reference) (InstigatedBy :type Controller%20Object%20Reference) (DamageCauser :type Actor%20Object%20Reference))
  (bind _mesh (Variables|Character|GetMesh))
  ;[0.05127 0.05127 0.05127] Health System
  (if (> (Variables|Default|GetHealth) 0.0)
    (Variables|Default|SetHealth (- (Variables|Default|GetHealth) Damage))
    (Audio|PlaySound2D "/Game/ShooterAI/SOunds/hitmarker.hitmarker" 1.0 1.0 0.0 0 0)
    (bind _asuisai_enemy_health (Utilities|Casting|CastToUISAI_EnemyHealth (UserInterface|GetWidget (Variables|Default|GetHealthbar%20Widget))))
    (Progress|SetPercent (Variables|/Game/ShooterAI/Interface/UISAI_EnemyHealth.UISAI_EnemyHealth_C|Gethealthbar _asuisai_enemy_health) (/ (Variables|Default|GetHealth) 1e+02))
    (if (<= (Variables|Default|GetHealth) 0.0)
      (Physics|SetSimulatePhysics _mesh true)
      (Class|SkeletalMeshComponent|SetPhysicsBlendWeight _mesh 1.0)
      (Collision|SetCollisionEnabled _mesh "QueryAndPhysics")
      (Utilities|FlowControl|Delay 2.0)
      (Actor|DestroyActor))))

(event Collision|EventActorBeginOverlap
  (params (OtherActor :type Actor%20Object%20Reference)))

(event EventTick
  (params (DeltaSeconds :type Float%20%28single-precision%29))
  (bind _healthbar_widget (Variables|Default|GetHealthbar%20Widget))
  ;[0.05127 0.05127 0.05127] Health System
  (Transformation|SetWorldRotation _healthbar_widget (Math|Rotator|FindLookatRotation (Transformation|GetWorldLocation _healthbar_widget) (Transformation|GetWorldLocation (Variables|/Script/Engine.PlayerCameraManager|GetTransformComponent (Game|GetPlayerCameraManager 0)))) false false))

(event EventBeginPlay)

(fn ConstructionScript)